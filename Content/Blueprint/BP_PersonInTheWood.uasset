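; One-shot scare-style event actor: a configurable skeletal-mesh figure appears with a sound when the player enters its trigger box.
; Tick moves the Arrow along SplinePath at fixed height; the construction script applies mesh, animation and trigger bounds.
; Optionally, the player is made to look at it, then it self-destroys after a delay.
; The end-of-path destroy compares speed, not travelled distance, to spline length, and any first overlap consumes the DoOnce.
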(event OnComponentBeginOverlap(TriggerBox)
  (params (OverlappedComponent :type Primitive%20Component%20Object%20Reference) (OtherActor :type Actor%20Object%20Reference) (OtherComp :type Primitive%20Component%20Object%20Reference) (OtherBodyIndex :type Integer) (bFromSweep :type Boolean) (SweepResult :type Hit%20Result%20Structure%20%28by%20ref%29))
  (Utilities|FlowControl|DoOnce false
    (:Completed
      (if (== OtherActor (Variables|Default|GetPlayerRef))
        (Variables|Default|SetTriggerAnim? true)
        (Development|SetHiddeninGame (Variables|Default|GetMovingEntity) false false)
        (Audio|SpawnSoundAttached (Variables|CharacterVariables|GetSoundToPlay) (Variables|Default|GetArrow) "None" "0, 0, 0" "0, 0, 0" "KeepRelativeOffset" false 1.0 1.0 0.0 0 0)
        (if (Variables|PlayerBehaviour|GetPlayerNeedToLook?)
          (Default|LookatEvent (Variables|Default|GetPlayerRef) self (Variables|PlayerBehaviour|GetLookAtTime))
          (Utilities|FlowControl|Delay (Variables|CharacterVariables|GetDuration))
          (Actor|DestroyActor))))))

(event EventBeginPlay
  (bind _splinepath (Variables|Default|GetSplinePath))
  (bind _arrow (Variables|Default|GetArrow))
  (bind _returnvalue (Spline|GetTransformatDistanceAlongSpline _splinepath 0.0 "World" false))
  (bind _asbp_first_person_character (Utilities|Casting|CastToBP_FirstPersonCharacter (Game|GetPlayerCharacter 0)))
  (Variables|Default|SetPlayerRef _asbp_first_person_character)
  (Transformation|SetWorldTransform _arrow (Math|Transform|MakeTransform (Math|Vector|MakeVector (.x (.location _returnvalue)) (.y (.location _returnvalue)) (.z (Transformation|GetWorldLocation _arrow))) (.rotation _returnvalue)) false false)
  (Development|SetHiddeninGame (Variables|Default|GetArrow) true true))

(event EventTick
  (params (DeltaSeconds :type Float%20%28single-precision%29))
  (bind _arrow (Variables|Default|GetArrow))
  (if (Variables|Default|GetTriggerAnim?)
    (Variables|Default|SetDistanceOnSpline (+ (* DeltaSeconds (Variables|CharacterVariables|GetSpeedOnSpline)) (Variables|Default|GetDistanceOnSpline)))
    (Transformation|SetWorldTransform _arrow (Math|Transform|MakeTransform (Math|Vector|MakeVector (.x (.location (Spline|GetTransformatDistanceAlongSpline (Variables|Default|GetSplinePath) (Variables|Default|GetDistanceOnSpline) "World" false))) (.y (.location (Spline|GetTransformatDistanceAlongSpline (Variables|Default|GetSplinePath) (Variables|Default|GetDistanceOnSpline) "World" false))) (.z (Transformation|GetWorldLocation _arrow))) (.rotation (Spline|GetTransformatDistanceAlongSpline (Variables|Default|GetSplinePath) (Variables|Default|GetDistanceOnSpline) "World" false))) false false)
    (if (>= (Variables|CharacterVariables|GetSpeedOnSpline) (Spline|GetSplineLength (Variables|Default|GetSplinePath)))
      (Variables|Default|SetTriggerAnim? false)
      (Actor|DestroyActor))))

(fn ConstructionScript
  (bind _movingentity (Variables|Default|GetMovingEntity))
  (bind _triggerbox (Variables|Default|GetTriggerBox))
  (Components|SkeletalMesh|SetSkeletalMeshAsset _movingentity (Variables|CharacterVariables|GetMeshDisplayed))
  (Class|SkeletalMeshComponent|SetAnimClass _movingentity (Variables|CharacterVariables|GetAnimClass))
  (Transformation|SetRelativeLocation _triggerbox (Variables|TriggerBoxVariables|GetTriggerBoxLocation) false false)
  (Transformation|SetRelativeScale3D _triggerbox (Variables|TriggerBoxVariables|GetTriggerBoxSize)))