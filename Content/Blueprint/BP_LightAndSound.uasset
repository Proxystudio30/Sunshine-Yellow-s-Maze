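; BP_LightAndSound is a one-shot horror trigger that plays a sound, switches lights to the opposite of their starting visibility, or both.
; BeginPlay caches the horror character, assigns the sound and sets initial light visibility, while the construction script places the trigger box and sound source.
; The first overlap fires the effects enabled by flags and can make the player look at this actor.
; DoOnce precedes the actor check, and light Delays sit inside loops.
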(event OnComponentBeginOverlap(TriggerBox)
  (params (OverlappedComponent :type Primitive%20Component%20Object%20Reference) (OtherActor :type Actor%20Object%20Reference) (OtherComp :type Primitive%20Component%20Object%20Reference) (OtherBodyIndex :type Integer) (bFromSweep :type Boolean) (SweepResult :type Hit%20Result%20Structure%20%28by%20ref%29))
  (Utilities|FlowControl|DoOnce false
    (:Completed
      (if (== OtherActor 0)
        (if (Variables|SoundVariables|GetUseSound?)
          (if (Variables|LightVariables|GetUseLight?)
            (Audio|Components|Audio|Play (Variables|Default|GetSoundSource) (Variables|SoundVariables|GetDelayBeforeSound))
            (for _array_element (Variables|LightVariables|GetLight)
              (Utilities|FlowControl|Delay (Variables|LightVariables|GetDelayBeforeLight))
              (Rendering|SetVisibility (Variables|/Script/Engine.Actor|GetRootComponent _array_element) (not (Variables|LightVariables|GetStartLightOn?)) false))
            (else
              (Audio|Components|Audio|Play (Variables|Default|GetSoundSource) (Variables|SoundVariables|GetDelayBeforeSound))))
          (if (Variables|PlayerBehaviour|GetPlayerNeedToLook?) :!label _label
            (Default|LookatEvent (Variables|Default|GetPlayerRef) self (Variables|PlayerBehaviour|GetLook%20at%20Time)))
          (elif (Variables|LightVariables|GetUseLight?)
            (for (_array_element_2 _array_index) (Variables|LightVariables|GetLight)
              (Utilities|FlowControl|Delay (Variables|LightVariables|GetDelayBeforeLight))
              (Development|PrintString (Utilities|String|ToString(Integer) _array_index))
              (Rendering|SetVisibility (Variables|/Script/Engine.Actor|GetRootComponent _array_element_2) (not (Variables|LightVariables|GetStartLightOn?)) false))
            (goto _label)
            (else
              (Development|PrintString "Not using any light or sound"))))))))

(event EventBeginPlay
  (bind _asbp_horror_character (Utilities|Casting|CastToBP_HorrorCharacter (Game|GetPlayerCharacter 0)))
  (Variables|Default|SetPlayerRef _asbp_horror_character)
  (Audio|Components|Audio|SetSound (Variables|Default|GetSoundSource) (Variables|SoundVariables|GetSoundToPlay))
  (for _array_element (Variables|LightVariables|GetLight)
    (Rendering|SetVisibility (Variables|/Script/Engine.Light|GetLightComponent _array_element) (Variables|LightVariables|GetStartLightOn?) false)))

(fn ConstructionScript
  (bind _triggerbox (Variables|Default|GetTriggerBox))
  (Transformation|SetRelativeLocation _triggerbox (Variables|TriggerBoxVariables|GetTriggerBoxLocation) false false)
  (Transformation|SetRelativeScale3D _triggerbox (Variables|TriggerBoxVariables|GetTriggerBoxSize))
  (Transformation|SetRelativeLocation (Variables|Default|GetSoundSource) (Variables|SoundVariables|GetSoundSourceLocation) false false))