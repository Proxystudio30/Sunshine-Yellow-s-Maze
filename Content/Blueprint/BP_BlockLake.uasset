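; BP_BlockLake is a trigger actor that plays a 2D voice line when the first-person player character enters its volumes.
; Box and sphere overlaps share one path that checks against the cached player reference and plays the configured sound.
; A DoOnce gate, reset after a cooldown delay, prevents rapid repeats.
; The construction script places and sizes both triggers from variables, allowing per-instance setup.
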(event OnComponentBeginOverlap(TriggerSphere)
  (params (OverlappedComponent :type Primitive%20Component%20Object%20Reference) (OtherActor :type Actor%20Object%20Reference) (OtherComp :type Primitive%20Component%20Object%20Reference) (OtherBodyIndex :type Integer) (bFromSweep :type Boolean) (SweepResult :type Hit%20Result%20Structure%20%28by%20ref%29))
  (if (or (== OverlappedComponent (Variables|Default|GetPlayer%20Ref)) (== (stale OnComponentBeginOverlap(TriggerBox) OtherActor) (Variables|Default|GetPlayer%20Ref)))
    (Utilities|FlowControl|DoOnce false
      (:Completed
        (Audio|PlaySound2D (Variables|VoiceLineVariables|GetSoundToPlay) 1.0 1.0 0.0 0 0)
        (Utilities|FlowControl|Delay (Variables|VoiceLineVariables|GetVoiceLineCooldown))
        (CallFunction|ResetVoiceLine)))))

(event OnComponentBeginOverlap(TriggerBox)
  (params (OverlappedComponent :type Primitive%20Component%20Object%20Reference) (OtherActor :type Actor%20Object%20Reference) (OtherComp :type Primitive%20Component%20Object%20Reference) (OtherBodyIndex :type Integer) (bFromSweep :type Boolean) (SweepResult :type Hit%20Result%20Structure%20%28by%20ref%29))
  (if (or (== (stale OnComponentBeginOverlap(TriggerSphere) OverlappedComponent) (Variables|Default|GetPlayer%20Ref)) (== OtherActor (Variables|Default|GetPlayer%20Ref)))
    (Utilities|FlowControl|DoOnce false
      (:Completed
        (Audio|PlaySound2D (Variables|VoiceLineVariables|GetSoundToPlay) 1.0 1.0 0.0 0 0)
        (Utilities|FlowControl|Delay (Variables|VoiceLineVariables|GetVoiceLineCooldown))
        (CallFunction|ResetVoiceLine)))))

(event Custom|ResetVoiceLine
  (Utilities|FlowControl|DoOnce false) ; enters at Reset
)

(event EventBeginPlay
  (bind _asbp_first_person_character (Utilities|Casting|CastToBP_FirstPersonCharacter (Game|GetPlayerCharacter 0)))
  (Variables|Default|SetPlayer%20Ref _asbp_first_person_character))

(fn ConstructionScript
  (bind _triggerbox (Variables|Default|GetTriggerBox))
  (bind _triggersphere (Variables|Default|GetTriggerSphere))
  (Transformation|SetRelativeLocation _triggerbox (Variables|TriggerBoxVariables|GetTriggerBoxLocation) false false)
  (Transformation|SetRelativeScale3D _triggerbox (Variables|TriggerBoxVariables|GetTriggerBoxSize))
  (Transformation|SetRelativeLocation _triggersphere (Variables|TriggerSphereVariables|GetTriggerSphereLocation) false false)
  (Components|Sphere|SetSphereRadius _triggersphere (Variables|TriggerSphereVariables|GetTriggerSphereRadius) true))