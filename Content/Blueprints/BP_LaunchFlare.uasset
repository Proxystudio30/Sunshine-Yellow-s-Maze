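; BP_LaunchFlare is a placeable trigger that launches a BP_Flare from an arrow when the player overlaps its box.
; The flare receives configurable speed and lifetime, carries an attached sound, and can optionally make the player look at it for a set time.
; A DoOnce precedes the player check, so the first overlap by any actor consumes it.
; The construction script exposes box and arrow transforms through variables.
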(event OnComponentBeginOverlap(TriggerBox)
  (params (OverlappedComponent :type Primitive%20Component%20Object%20Reference) (OtherActor :type Actor%20Object%20Reference) (OtherComp :type Primitive%20Component%20Object%20Reference) (OtherBodyIndex :type Integer) (bFromSweep :type Boolean) (SweepResult :type Hit%20Result%20Structure%20%28by%20ref%29))
  (Utilities|FlowControl|DoOnce false
    (:Completed
      (if (== OtherActor (Variables|Default|GetPlayerRef))
        (bind _returnvalue (Game|SpawnActorfromClass "/Game/Blueprints/BP_Flare.BP_Flare_C" (Transformation|GetWorldTransform (Variables|Default|GetLaunchArrow)) "Undefined" "MultiplyWithRoot" 0 (Variables|LauncherVariables|GetInitialProjectileSpeed) (Variables|LauncherVariables|GetMaxProjectileSpeed) (Variables|LauncherVariables|GetProjectileLifeTime) 0))
        (Audio|SpawnSoundAttached (Variables|LauncherVariables|GetSoundToPlay) (Variables|/Game/Blueprints/BP_Flare.BP_Flare_C|GetSphere _returnvalue) "None" "0, 0, 0" "0, 0, 0" "KeepRelativeOffset" false 1.0 1.0 0.0 0 0)
        (if (Variables|PlayerBehaviour|GetPlayerNeedToLook?)
          (Default|LookatEvent (Variables|Default|GetPlayerRef) _returnvalue (Variables|PlayerBehaviour|GetLook%20at%20Time)))))))

(event EventBeginPlay
  (bind _asbp_first_person_character (Utilities|Casting|CastToBP_FirstPersonCharacter (Game|GetPlayerCharacter 0)))
  (Variables|Default|SetPlayerRef _asbp_first_person_character))

(fn ConstructionScript
  (bind _triggerbox (Variables|Default|GetTriggerBox))
  (bind _launcharrow (Variables|Default|GetLaunchArrow))
  (Transformation|SetRelativeLocation _triggerbox (Variables|TriggerBoxVariables|GetTriggerBoxLocation) false false)
  (Transformation|SetRelativeScale3D _triggerbox (Variables|TriggerBoxVariables|GetTriggerBoxSize))
  (Transformation|SetRelativeLocation _launcharrow (Variables|LauncherVariables|GetLaunchArrowLocation) false false)
  (Transformation|SetRelativeRotation _launcharrow (Variables|LauncherVariables|GetLaunchArrowRotation) false false))